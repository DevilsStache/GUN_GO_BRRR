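; Key-locked swinging door with a status light that reacts when the player enters or leaves its trigger zone.
; BeginPlay caches the first-person player and gives the light mesh a dynamic emissive material instance.
; On overlap the light brightens, turning green and playing a timeline that rotates the door open if the player's HasKey is set, otherwise turning red.
; Leaving restores the default light and reverses the timeline.
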(event OnComponentBeginOverlap(Door_Triggerzone)
  (params (OverlappedComponent :type Primitive%20Component%20Object%20Reference) (OtherActor :type Actor%20Object%20Reference) (OtherComp :type Primitive%20Component%20Object%20Reference) (OtherBodyIndex :type Integer) (bFromSweep :type Boolean) (SweepResult :type Hit%20Result%20Structure%20%28by%20ref%29))
  ;[1 1 1 1 50] Light colour change
  (if (== OtherActor (Variables|Default|GetPlayer_Reference))
    (Rendering|Material|SetScalarParameterValue (Variables|Default|GetDynamicMaterial) "Intensity" 1e+02 :!class /Script/Engine.MaterialInstanceDynamic)
    (if (Variables|/Game/FirstPerson/Blueprints/BP_FirstPersonCharacter.BP_FirstPersonCharacter_C|GetHasKey (Variables|Default|GetPlayer_Reference))
      (Rendering|Material|SetVectorParameterValue (Variables|Default|GetDynamicMaterial) "Colour" "(R=0.160640,G=1.000000,B=0.000000,A=1.000000)" :!class /Script/Engine.MaterialInstanceDynamic)
      ;[1 1 1] Door opening
      (bind _door (Timeline|Timeline%20Door_open_close Play)
        (:Update
          (Variables|Default|SetDoor_Opening true)
          (Transformation|SetRelativeRotation (Variables|Default|GetSM_Door) (Math|Rotator|Lerp(Rotator) "0, 0, 0" "-90.000000,0.000000,0.000000" _door) false false))
        (:Finished
          (Variables|Default|SetDoor_Opening false)))
      (else
        (Rendering|Material|SetVectorParameterValue (Variables|Default|GetDynamicMaterial) "Colour" "(R=1.000000,G=0.000000,B=0.006044,A=1.000000)" :!class /Script/Engine.MaterialInstanceDynamic)))))

(event OnComponentEndOverlap(Door_Triggerzone)
  (params (OverlappedComponent :type Primitive%20Component%20Object%20Reference) (OtherActor :type Actor%20Object%20Reference) (OtherComp :type Primitive%20Component%20Object%20Reference) (OtherBodyIndex :type Integer))
  ;[1 1 1 1 34] Return to Default
  (if (== OtherActor (Variables|Default|GetPlayer_Reference))
    (Rendering|Material|SetScalarParameterValue (Variables|Default|GetDynamicMaterial) "Intensity" 1.0 :!class /Script/Engine.MaterialInstanceDynamic)
    (Rendering|Material|SetVectorParameterValue (Variables|Default|GetDynamicMaterial) "Colour" "(R=1.000000,G=0.301961,B=0.200000,A=1.000000)" :!class /Script/Engine.MaterialInstanceDynamic)
    ;[1 1 1] Door opening
    (bind _door (Timeline|Timeline%20Door_open_close Reverse)
      (:Update
        (Variables|Default|SetDoor_Opening true)
        (Transformation|SetRelativeRotation (Variables|Default|GetSM_Door) (Math|Rotator|Lerp(Rotator) "0, 0, 0" "-90.000000,0.000000,0.000000" _door) false false))
      (:Finished
        (Variables|Default|SetDoor_Opening false)))))

(event EventBeginPlay
  ;[1 1 1] the whole tyhing
  (Utilities|FlowControl|Sequence
    (:then_0
      ;;[1 1 1] Player character ref
      (bind _asbp_first_person_character (Utilities|Casting|CastToBP_FirstPersonCharacter (Game|GetPlayerCharacter 0)))
      (Variables|Default|SetPlayer_Reference _asbp_first_person_character))
    (:then_1
      ;;[1 0.1093 0.2694 1 42] Set up material
      (bind _returnvalue (Rendering|Material|CreateDynamicMaterialInstance "/Game/Target_Practice/Materials/MI_DoorEmission.MI_DoorEmission" "None" "None" :!class /Script/Engine.KismetMaterialLibrary))
      (bind _output_get (Variables|Default|SetDynamicMaterial _returnvalue))
      (Rendering|Material|SetMaterial (Variables|Default|GetSM_Light) 0 _output_get))))

(fn ConstructionScript)