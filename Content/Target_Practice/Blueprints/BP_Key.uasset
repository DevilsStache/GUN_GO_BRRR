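; BP_Key is a key pickup that stays hidden and non-collidable until no BP_targetmove actors remain in the level.
; Each Tick gathers those actors and uses the index returned by an array Add as their count, toggling visibility and collision.
; A DoOnce plays steam particles and sound when the key first appears.
; Player overlap with the capsule sets HasKey on BP_FirstPersonCharacter, plays a sound and destroys the key.
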(event OnComponentBeginOverlap(Capsule_Colider)
  (params (OverlappedComponent :type Primitive%20Component%20Object%20Reference) (OtherActor :type Actor%20Object%20Reference) (OtherComp :type Primitive%20Component%20Object%20Reference) (OtherBodyIndex :type Integer) (bFromSweep :type Boolean) (SweepResult :type Hit%20Result%20Structure%20%28by%20ref%29))
  ;[1 0.8554 0.506 1 50] Key Pickup
  (if (== OtherActor (Variables|Default|GetPlayer_Reference))
    (Variables|/Game/FirstPerson/Blueprints/BP_FirstPersonCharacter.BP_FirstPersonCharacter_C|SetHasKey (Variables|Default|GetPlayer_Reference) true)
    (Audio|PlaySoundatLocation "/Game/StarterContent/Audio/Light02.Light02" (Transformation|GetActorLocation) "0, 0, 0" 1.0 1.0 0.0 0 0 0 0)
    (Actor|DestroyActor)))

(event EventBeginPlay
  ;[0.3153 0.3519 1 1 50] Set up
  (bind _asbp_first_person_character (Utilities|Casting|CastToBP_FirstPersonCharacter (Game|GetPlayerCharacter 0)))
  (Variables|Default|SetPlayer_Reference _asbp_first_person_character))

(event EventTick
  (params (DeltaSeconds :type Float%20%28single-precision%29))
  (bind _key (Variables|Default|GetKey))
  (bind _returnvalue (Transformation|GetWorldLocation _key))
  ;[1 0.04167 0.04167 1 57] Key Visablility
  (bind _outactors (Actor|GetAllActorsOfClass "/Game/Target_Practice/Blueprints/BP_targetmove.BP_targetmove_C"))
  (bind _returnvalue_2 (Utilities|Array|Add _outactors 0))
  (Utilities|FlowControl|Sequence
    (:then_0
      (Rendering|SetVisibility (Variables|Default|GetKey) (<= _returnvalue_2 0) true)
      (Collision|SetActorEnableCollision (<= _returnvalue_2 0))
      ;[1 1 1 1 58] Key spawn effects
      (if (<= _returnvalue_2 0)
        (Utilities|FlowControl|DoOnce false
          (:Completed
            (Effects|SpawnEmitteratLocation "/Game/StarterContent/Particles/P_Steam_Lit.P_Steam_Lit" _returnvalue)
            (Audio|PlaySoundatLocation "/Game/StarterContent/Audio/Steam01_Cue.Steam01_Cue" _returnvalue "0, 0, 0" 1.0 1.0 0.0 0 0 0 0)))))))

(fn ConstructionScript)