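; BP_targetmove is a shootable target actor for target practice that moves back and forth.
; Tick offsets it along the normalized Direction by Speed each frame, not scaled by delta time, while a looping MovementDuration timer reverses Direction.
; Each Hit event subtracts a hitpoint and plays a sound at the impact location; at zero it spawns an explosion, plays a fire sound and destroys itself.
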(event Custom|Flip%20Direction
  ;[0.1816 1 0.351] Flip Direction
  (Variables|Default|SetDirection (* (Variables|Default|GetDirection) -1.0)))

(event EventBeginPlay
  ;[0.1816 1 0.351] Flip Direction
  (Utilities|Time|SetTimerbyEvent (delegate Custom|Flip%20Direction) (Variables|Default|GetMovement_Duration) true))

(event EventTick
  (params (DeltaSeconds :type Float%20%28single-precision%29))
  ;[0.3241 0.6785 1] target movement
  (Transformation|AddActorWorldOffset (* (Math|Vector|Normalize (Variables|Default|GetDirection)) (Variables|Default|GetSpeed))))

(event Collision|EventHit
  (params (MyComp :type Primitive%20Component%20Object%20Reference) (Other :type Actor%20Object%20Reference) (OtherComp :type Primitive%20Component%20Object%20Reference) (bSelfMoved :type Boolean) (HitLocation :type Vector :default "0, 0, 0") (HitNormal :type Vector :default "0, 0, 0") (NormalImpulse :type Vector :default "0, 0, 0") (Hit :type Hit%20Result%20Structure%20%28by%20ref%29))
  ;[1 0.5042 0.4444] Hidden Check
  (Variables|Default|SetHitpoints (- (Variables|Default|GetHitpoints) 1))
  (if (<= (Variables|Default|GetHitpoints) 0)
    ;[1 0.6125 0.8466] Destroy
    (Effects|SpawnEmitteratLocation "/Game/StarterContent/Particles/P_Explosion.P_Explosion" HitLocation)
    (Audio|PlaySoundatLocation "/Game/StarterContent/Audio/Fire01.Fire01" HitLocation "0, 0, 0" 1.0 1.0 0.0 0 0 0 0)
    (Actor|DestroyActor)
    (else
      (Audio|PlaySoundatLocation "/Game/StarterContent/Audio/Light02.Light02" HitLocation "0, 0, 0" 1.0 1.0 0.0 0 0 0 0))))

(fn ConstructionScript)